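; PCM_Test is a player camera manager Blueprint for blending between two cameras, taking its default aspect ratio from the BP_Plane pawn's camera.
; TriggerCameraTransition plays a timeline that interpolates world location and rotation from start to target camera.
; BlueprintUpdateCamera outputs that transform with the view target's FOV, using InTransition as the override flag.
; InTransition is only ever set false here, so this file never enables the override.
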(event `self.ReceiveBeginPlay`
  (bind _asbp_plane (cast `/Game/Blueprints/Pawn/BP_Plane` (`GameplayStatics.GetPlayerPawn` 0)))
  (set `self.DefaultAspectRatio` (`CameraComponent.AspectRatio` (`/Game/Blueprints/Pawn/BP_Plane.Camera` _asbp_plane))))

(event `TriggerCameraTransition`
  (params (StartCamera :type "CameraComponent Object Reference") (TargetCamera :type "CameraComponent Object Reference"))
  (set `self.InTransition` false)
  (bind (_direction _alphacurve) (`Timeline|CameraTransition` :!via `PlayFromStart`)
    (:`Update`
      (set `self.PositionTransition` (`KismetMathLibrary.VLerp` (`SceneComponent.K2_GetComponentLocation` StartCamera) (`SceneComponent.K2_GetComponentLocation` TargetCamera) _alphacurve))
      (set `self.RotationTransition` (`KismetMathLibrary.RLerp` (`SceneComponent.K2_GetComponentRotation` StartCamera) (`SceneComponent.K2_GetComponentRotation` TargetCamera) _alphacurve)))
    (:`Finished`
      (set `self.InTransition` false))))

(fn `BlueprintUpdateCamera`
  (params (CameraTarget :type "Actor Object Reference"))
  (returns (NewCameraLocation :type "Vector Structure") (NewCameraRotation :type "Rotator Structure") (NewCameraFOV :type "Float (single-precision)") (ReturnValue :type Boolean))
  (return (`self.PositionTransition`) (`self.RotationTransition`) (`CameraComponent.FieldOfView` (`self.GetComponentByClass` CameraTarget "/Script/Engine.CameraComponent")) (`self.InTransition`)))

(fn `UserConstructionScript`)