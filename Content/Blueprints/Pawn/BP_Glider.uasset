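; BP_Glider is a glider pawn Blueprint that drives speed-line and thruster visual feedback.
; On BeginPlay it adds the WBP_SpeedLines widget to the viewport, swaps its brush to a dynamic material instance and pauses two Niagara thrust effects.
; Starting the IA_Thrust input resets both effects.
; Each tick, a curve maps ForwardSpeed to the speed-line material's opacity.
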(event `self.ReceiveBeginPlay`
  (bind _brush (`Image.Brush` (`/Game/Blueprints/Widget/WBP_SpeedLines.SpeedLines` (`self.SpeedLines`))))
  (bind _returnvalue (`|CreateWidget` "/Game/Blueprints/Widget/WBP_SpeedLines.WBP_SpeedLines_C"))
  (bind _output_get (set `self.SpeedLines` _returnvalue))
  (`UserWidget.AddToViewport` _output_get 0)
  (bind _returnvalue_2 (`KismetMaterialLibrary.CreateDynamicMaterialInstance` (`WidgetBlueprintLibrary.GetBrushResourceAsMaterial` _brush)))
  (bind _output_get_2 (set `self.SpeedLinesMat` _returnvalue_2))
  (`WidgetBlueprintLibrary.SetBrushResourceToMaterial` _brush _output_get_2)
  (`NiagaraComponent.SetPaused` (`self.NS_Thrust1`) true)
  (`NiagaraComponent.SetPaused` (`self.NS_Thrust`) true))

(event `EnhancedInput|/Game/Inputs/InputActions/IA_Thrust`
  (params (ActionValue :type Boolean) (ElapsedSeconds :type "Float (double-precision)") (TriggeredSeconds :type "Float (double-precision)") (InputAction :type "InputAction Object Reference" :default "/Game/Inputs/InputActions/IA_Thrust.IA_Thrust"))
  (:`Started`
    (`NiagaraComponent.ResetSystem` (`self.NS_Thrust1`))
    (`NiagaraComponent.ResetSystem` (`self.NS_Thrust`))))

(event `self.ReceiveTick`
  (params (DeltaSeconds :type "Float (single-precision)"))
  (`MaterialInstanceDynamic.SetScalarParameterValue` (`self.SpeedLinesMat`) "Opacity" (`CurveFloat.GetFloatValue` (`self.C_SpeedLinesOpacity`) (`self.ForwardSpeed`))))

(fn `UserConstructionScript`)