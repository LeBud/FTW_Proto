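; Player-controlled plane pawn with a simplified physics-driven flight model acting on its Master component.
; Enhanced Input applies accelerations for thrust and pitch, roll and yaw torques, and drives camera look.
; Each tick applies manual gravity and counter-torque damping, updates velocity and an angle-of-attack value, then adds speed-squared drag and lift with debug lines.
; AoA dots forward against a vector built from speed alone, not velocity direction.
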(event `self.ReceiveBeginPlay`
  ;[0.15 0 0 0.5] Input Binding
  (bind _asplayer_controller (cast `PlayerController` (`self.GetController`)))
  (bind _returnvalue (pcsubsystem `EnhancedInputLocalPlayerSubsystem` _asplayer_controller))
  (`/Engine/EditorBlueprintResources/StandardMacros.IsValid` _returnvalue
    (:`Is Valid`
      (`EnhancedInputSubsystemInterface.AddMappingContext` _returnvalue "/Game/Inputs/IMC_Plane.IMC_Plane" 0 (struct)))))

(event `self.ReceiveTick`
  (params (DeltaSeconds :type "Float (single-precision)"))
  (`self.HandleGravity`)
  (`self.RotationCompensation`)
  (`self.UpdateState`)
  (`self.UpdateDrag`)
  (`self.UpdateLift`))

(event `EnhancedInput|/Game/Inputs/InputActions/IA_Look`
  (params (ActionValue :type "Vector2D Structure") (ElapsedSeconds :type "Float (double-precision)") (TriggeredSeconds :type "Float (double-precision)") (InputAction :type "InputAction Object Reference" :default "/Game/Inputs/InputActions/IA_Look.IA_Look"))
  ;[0.002344 0.15 0.01015 0.5] Camera Inputs
  (:`Triggered`
    (`self.AddControllerYawInput` ActionValue_X)
    (`self.AddControllerPitchInput` ActionValue_Y)))

(event `EnhancedInput|/Game/Inputs/InputActions/IA_Roll`
  (params (ActionValue :type "Float (double-precision)") (ElapsedSeconds :type "Float (double-precision)") (TriggeredSeconds :type "Float (double-precision)") (InputAction :type "InputAction Object Reference" :default "/Game/Inputs/InputActions/IA_Roll.IA_Roll"))
  ;[0 0.0482 0.15 0.5] Input - Rotation Function
  (:`Triggered`
    (bind _result (`/Engine/EditorBlueprintResources/StandardMacros.NegateFloat` ActionValue)
      (:`  `
        (`self.HandleInputRotation` _result (`self.RollForce`) (`SceneComponent.GetForwardVector` (`self.Master`)))))))

(event `EnhancedInput|/Game/Inputs/InputActions/IA_Thrust`
  (params (ActionValue :type Boolean) (ElapsedSeconds :type "Float (double-precision)") (TriggeredSeconds :type "Float (double-precision)") (InputAction :type "InputAction Object Reference" :default "/Game/Inputs/InputActions/IA_Thrust.IA_Thrust"))
  (bind _master (`self.Master`))
  (:`Triggered`
    (`PrimitiveComponent.AddForce` _master (* (`SceneComponent.GetForwardVector` _master) 10000.0) "None" true)))

(event `EnhancedInput|/Game/Inputs/InputActions/IA_Pitch`
  (params (ActionValue :type "Float (double-precision)") (ElapsedSeconds :type "Float (double-precision)") (TriggeredSeconds :type "Float (double-precision)") (InputAction :type "InputAction Object Reference" :default "/Game/Inputs/InputActions/IA_Pitch.IA_Pitch"))
  ;[0 0.0482 0.15 0.5] Input - Rotation Function
  (:`Triggered`
    (`self.HandleInputRotation` ActionValue (`self.PitchForce`) (`SceneComponent.GetRightVector` (`self.Master`)))))

(event `EnhancedInput|/Game/Inputs/InputActions/IA_Yaw`
  (params (ActionValue :type "Float (double-precision)") (ElapsedSeconds :type "Float (double-precision)") (TriggeredSeconds :type "Float (double-precision)") (InputAction :type "InputAction Object Reference" :default "/Game/Inputs/InputActions/IA_Yaw.IA_Yaw"))
  ;[0 0.0482 0.15 0.5] Input - Rotation Function
  (:`Triggered`
    (`self.HandleInputRotation` ActionValue (`self.YawForce`) (`SceneComponent.GetUpVector` (`self.Master`)))))

(fn `HandleGravity`
  (bind _master (`self.Master`))
  (`PrimitiveComponent.AddForce` _master (* (`PrimitiveComponent.GetMass` _master) (0.0 0.0 -980.0)) "None" false))

(fn `HandleInputRotation`
  (params (`Input Value` :type "Float (double-precision)") (RotationForce :type "Float (double-precision)") (VectorDir :type "Vector Structure"))
  (`PrimitiveComponent.AddTorqueInDegrees` (`self.Master`) (`KismetMathLibrary.VLerp` (0.0 0.0 0.0) (* VectorDir (* `Input Value` RotationForce)) 0.1) "None" true))

(fn `RotationCompensation`
  (`PrimitiveComponent.AddTorqueInDegrees` (`self.Master`) (/ (`KismetMathLibrary.NegateVector` (`PrimitiveComponent.GetPhysicsAngularVelocityInDegrees` (`self.Master`) "None")) (`self.Angular Compensation`)) "None" true))

(fn `UpdateDrag`
  (locals (DragDir :type "Vector Structure") (DragForceMag :type "Float (double-precision)"))
  (bind _master (`self.Master`))
  (bind _speed (`self.Speed`))
  (bind _returnvalue (`SceneComponent.K2_GetComponentLocation` _master))
  (bind _returnvalue_2 (* (`local.DragDir`) (`local.DragForceMag`)))
  (set `local.DragDir` (`KismetMathLibrary.Normal` (`KismetMathLibrary.NegateVector` (`self.Velocity`))))
  (set `local.DragForceMag` (* 0.5 (`self.AirDensity`) _speed _speed (`self.DragCoef`) (`self.Area`)))
  (`PrimitiveComponent.AddForce` _master _returnvalue_2 "None" false)
  (`KismetSystemLibrary.DrawDebugLine` _returnvalue (+ _returnvalue _returnvalue_2) (struct :`G` 0.036409 :`B` 1.0 :`A` 1.0)))

(fn `UpdateLift`
  (locals (LiftDir :type "Vector Structure") (LiftForceMag :type "Float (double-precision)"))
  (bind _master (`self.Master`))
  (bind _speed (`self.Speed`))
  (bind _returnvalue (`SceneComponent.K2_GetComponentLocation` _master))
  (bind _returnvalue_2 (* (`local.LiftDir`) (`local.LiftForceMag`)))
  (set `local.LiftDir` (`KismetMathLibrary.Normal` (`KismetMathLibrary.Cross_VectorVector` (`KismetMathLibrary.Normal` (`self.Velocity`)) (`SceneComponent.GetRightVector` (`self.Master`)))))
  (set `self.LiftCoefficient` (`KismetMathLibrary.FClamp` (* (`self.AoA`) 2.0) -1.5 1.5))
  (set `local.LiftForceMag` (* 0.5 (`self.AirDensity`) _speed _speed (`self.LiftCoefficient`) (`self.Area`)))
  (`PrimitiveComponent.AddForce` _master _returnvalue_2 "None" false)
  (`KismetSystemLibrary.DrawDebugLine` _returnvalue (+ _returnvalue _returnvalue_2) (struct :`R` 0.145561 :`G` 1.0 :`A` 1.0)))

(fn `UpdateState`
  (bind _master (`self.Master`))
  (bind _returnvalue (`PrimitiveComponent.GetPhysicsLinearVelocity` _master "None"))
  (bind _output_get (set `self.Velocity` _returnvalue))
  (bind _returnvalue_2 (`KismetMathLibrary.VSize` _output_get))
  (set `self.Speed` _returnvalue_2)
  (set `self.AoA` (`KismetMathLibrary.Acos` (`KismetMathLibrary.Dot_VectorVector` (`SceneComponent.GetForwardVector` _master) (`KismetMathLibrary.Conv_DoubleToVector` _returnvalue_2)))))

(fn `UserConstructionScript`)