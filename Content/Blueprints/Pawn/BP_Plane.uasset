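; Player-controlled plane pawn with a work-in-progress physics flight model driven by Enhanced Input.
; Input applies roll, pitch and yaw torques plus forward thrust, while Tick adds gravity and counter-torque damping.
; Tick also derives local velocities and angles of attack, computing per-axis drag for debug display only.
; Curve-based lift, rudder and induced drag are written but disconnected, as are the drag force and AddForwardForce.
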(event `self.ReceiveBeginPlay`
  ;[0.15 0 0 0.5] Input Binding
  (bind _asplayer_controller (cast `PlayerController` (`self.GetController`)))
  (bind _returnvalue (pcsubsystem `EnhancedInputLocalPlayerSubsystem` _asplayer_controller))
  (`/Engine/EditorBlueprintResources/StandardMacros.IsValid` _returnvalue
    (:`Is Valid`
      (`EnhancedInputSubsystemInterface.AddMappingContext` _returnvalue "/Game/Inputs/IMC_Plane.IMC_Plane" 0 (struct)))))

(event `self.ReceiveTick`
  (params (DeltaSeconds :type "Float (single-precision)"))
  (`self.HandleGravity`)
  (`self.HandleRotationCompensation`)
  (`self.CalculateState`)
  (`self.CalculateAngleOfAttack`)
  (`self.UpdateDrag` DeltaSeconds)
  (`self.CalculateState`)
  (`KismetSystemLibrary.PrintString` (`KismetStringLibrary.Concat_StrStr` "velocity" (`KismetStringLibrary.Conv_VectorToString` (`self.Velocity`))) true true (struct :`R` 1.0 :`G` 0.936135 :`A` 1.0) 2.0 "0")
  (`KismetSystemLibrary.PrintString` (`KismetStringLibrary.Concat_StrStr` "local velocity" (`KismetStringLibrary.Conv_VectorToString` (`self.LocalVelocity`))) true true (struct :`G` 1.0 :`B` 0.384904 :`A` 1.0) 2.0 "1")
  (`KismetSystemLibrary.PrintString` (`KismetStringLibrary.Concat_StrStr` "local angular velocity" (`KismetStringLibrary.Conv_VectorToString` (`self.LocalAngularVelocity`))) true true (struct :`G` 0.66 :`B` 1.0 :`A` 1.0) 2.0 "2"))

(event `EnhancedInput|/Game/Inputs/InputActions/IA_Look`
  (params (ActionValue :type "Vector2D Structure") (ElapsedSeconds :type "Float (double-precision)") (TriggeredSeconds :type "Float (double-precision)") (InputAction :type "InputAction Object Reference" :default "/Game/Inputs/InputActions/IA_Look.IA_Look"))
  ;[0.002344 0.15 0.01015 0.5] Camera Inputs
  (:`Triggered`
    (`self.AddControllerYawInput` ActionValue_X)
    (`self.AddControllerPitchInput` ActionValue_Y)))

(event `EnhancedInput|/Game/Inputs/InputActions/IA_Roll`
  (params (ActionValue :type "Float (double-precision)") (ElapsedSeconds :type "Float (double-precision)") (TriggeredSeconds :type "Float (double-precision)") (InputAction :type "InputAction Object Reference" :default "/Game/Inputs/InputActions/IA_Roll.IA_Roll"))
  ;[0 0.0482 0.15 0.5] Input - Rotation Function
  (:`Triggered`
    (bind _result (`/Engine/EditorBlueprintResources/StandardMacros.NegateFloat` ActionValue)
      (:`  `
        (`self.HandleInputRotation` _result (`self.RollForce`) (`SceneComponent.GetForwardVector` (`self.Master`)))))))

(event `EnhancedInput|/Game/Inputs/InputActions/IA_Pitch`
  (params (ActionValue :type "Float (double-precision)") (ElapsedSeconds :type "Float (double-precision)") (TriggeredSeconds :type "Float (double-precision)") (InputAction :type "InputAction Object Reference" :default "/Game/Inputs/InputActions/IA_Pitch.IA_Pitch"))
  ;[0 0.0482 0.15 0.5] Input - Rotation Function
  (:`Triggered`
    (`self.HandleInputRotation` ActionValue (`self.PitchForce`) (`SceneComponent.GetRightVector` (`self.Master`)))))

(event `EnhancedInput|/Game/Inputs/InputActions/IA_Yaw`
  (params (ActionValue :type "Float (double-precision)") (ElapsedSeconds :type "Float (double-precision)") (TriggeredSeconds :type "Float (double-precision)") (InputAction :type "InputAction Object Reference" :default "/Game/Inputs/InputActions/IA_Yaw.IA_Yaw"))
  ;[0 0.0482 0.15 0.5] Input - Rotation Function
  (:`Triggered`
    (`self.HandleInputRotation` ActionValue (`self.YawForce`) (`SceneComponent.GetUpVector` (`self.Master`)))))

(event `EnhancedInput|/Game/Inputs/InputActions/IA_Thrust`
  (params (ActionValue :type Boolean) (ElapsedSeconds :type "Float (double-precision)") (TriggeredSeconds :type "Float (double-precision)") (InputAction :type "InputAction Object Reference" :default "/Game/Inputs/InputActions/IA_Thrust.IA_Thrust"))
  (bind _master (`self.Master`))
  (:`Triggered`
    (`PrimitiveComponent.AddForce` _master (* (`SceneComponent.GetForwardVector` _master) 1000.0) "None" true)))

(event `EnhancedInput|/Game/Inputs/InputActions/IA_AirJump`
  (params (ActionValue :type Boolean) (ElapsedSeconds :type "Float (double-precision)") (TriggeredSeconds :type "Float (double-precision)") (InputAction :type "InputAction Object Reference" :default "/Game/Inputs/InputActions/IA_AirJump.IA_AirJump")))

(fn `AddForwardForce`
  (bind _master (`self.Master`))
  (bind _returnvalue (`PrimitiveComponent.GetPhysicsLinearVelocity` _master "None"))
  (`PrimitiveComponent.SetPhysicsLinearVelocity` (`self.Master`) (`KismetMathLibrary.VLerp` _returnvalue (* (`SceneComponent.GetForwardVector` _master) (`KismetMathLibrary.FClamp` (* (`self.EngineForce`) (`self.EngineMultForce`)) 0.0 25000.0)) 0.01) false "None"))

(fn `CalculateAngleOfAttack`
  (bind (_localvelocity_x _localvelocity_y) (`KismetMathLibrary.BreakVector` (`self.LocalVelocity`)))
  (bind (_localvelocity_x_2 _localvelocity_y_2 _localvelocity_z) (`KismetMathLibrary.BreakVector` (`self.LocalVelocity`)))
  (bind _result (`/Engine/EditorBlueprintResources/StandardMacros.NegateFloat` _localvelocity_z)
    (:`  `
      (set `self.AngleOfAttack` (`KismetMathLibrary.Atan2` _result _localvelocity_x_2))
      (set `self.AngleOfAttackYaw` (`KismetMathLibrary.Atan2` _localvelocity_y _localvelocity_x))
      (`KismetSystemLibrary.PrintText` (`|FormatText` "AOA {x}" (`self.AngleOfAttack`)) true true (struct :`R` 0.649839 :`B` 1.0 :`A` 1.0) 2.0 "aoa")
      (`KismetSystemLibrary.PrintText` (`|FormatText` "AOA YAW {x}" (`self.AngleOfAttackYaw`)) true true (struct :`R` 0.649839 :`B` 1.0 :`A` 1.0) 2.0 "aoay"))))

(fn `CalculateLift`
  (params (AngleOfAttack :type "Float (double-precision)") (Axis :type "Vector Structure") (liftPower :type "Float (double-precision)") (aoaCurve :type "CurveFloat Object Reference") (inducedDragCurve :type "CurveFloat Object Reference"))
  (returns (`return Value` :type "Vector Structure"))
  (locals (liftVelocity :type "Vector Structure" :default (0.0 0.0 0.0)) (v2 :type "Float (double-precision)" :default 0.0) (liftCoef :type "Float (single-precision)" :default 0.0) (LiftForce :type "Float (double-precision)") (liftDir :type "Vector Structure" :default (0.0 0.0 0.0)) (lift :type "Vector Structure") (dragForce :type "Float (double-precision)" :default 0.0) (dragDir :type "Vector Structure" :default (0.0 0.0 0.0)) (localInducedDrag :type "Vector Structure"))
  (bind _localvelocity_x (`KismetMathLibrary.BreakVector` (`self.LocalVelocity`)))
  (bind _output_get (set `local.liftVelocity` (`KismetMathLibrary.ProjectVectorOnToPlane` (`self.LocalVelocity`) Axis)))
  (set `local.v2` (/ (`KismetMathLibrary.VSizeSquared` _output_get) 100.0))
  (set `local.liftCoef` (`CurveFloat.GetFloatValue` aoaCurve (`KismetMathLibrary.RadiansToDegrees` AngleOfAttack)))
  (bind _output_get_2 (set `local.LiftForce` (* (`local.v2`) (`local.liftCoef`) liftPower)))
  (bind _output_get_3 (set `local.liftDir` (`KismetMathLibrary.Cross_VectorVector` (`KismetMathLibrary.Normal` (`local.liftVelocity`)) Axis)))
  (set `local.lift` (* _output_get_3 _output_get_2))
  (set `local.dragForce` (`KismetMathLibrary.Square` (`local.liftCoef`)))
  (bind _output_get_4 (set `local.dragDir` (`KismetMathLibrary.Normal` (`KismetMathLibrary.NegateVector` (`local.liftVelocity`)))))
  (set `local.localInducedDrag` (* _output_get_4 (`local.v2`) (`local.dragForce`) (`self.InducedDrag`) (`CurveFloat.GetFloatValue` inducedDragCurve (`KismetMathLibrary.FMax` 0.0 _localvelocity_x))))
  (return (+ (`local.lift`) (`local.localInducedDrag`))))

(fn `CalculateState`
  (locals (InverseRotation :type "Rotator Structure"))
  (bind _master (`self.Master`))
  (bind _returnvalue (`KismetMathLibrary.NegateRotator` (`SceneComponent.K2_GetComponentRotation` _master)))
  (bind (_returnvalue_x _returnvalue_y _returnvalue_z _returnvalue_w) (`KismetMathLibrary.BreakQuat` (`KismetMathLibrary.Conv_RotatorToQuaternion` _returnvalue)))
  (set `local.InverseRotation` _returnvalue)
  (`KismetSystemLibrary.PrintString` (`KismetTextLibrary.Conv_TextToString` (`|FormatText` "Quat x {x} y {y} z {z} w {w}" _returnvalue_x _returnvalue_y _returnvalue_z _returnvalue_w)) true true (struct :`R` 1.0 :`B` 0.150339 :`A` 1.0) 2.0 "quat")
  (bind _returnvalue_2 (`PrimitiveComponent.GetPhysicsLinearVelocity` _master "None"))
  (bind _output_get (set `self.Velocity` _returnvalue_2))
  (set `self.LocalVelocity` (`KismetMathLibrary.Quat_RotateVector` (`KismetMathLibrary.Conv_RotatorToQuaternion` (`local.InverseRotation`)) _output_get))
  (set `self.LocalAngularVelocity` (`KismetMathLibrary.Quat_RotateVector` (`KismetMathLibrary.Conv_RotatorToQuaternion` (`local.InverseRotation`)) (`PrimitiveComponent.GetPhysicsAngularVelocityInRadians` _master "None"))))

(fn `CalculateSteering`)

(fn `HandleGravity`
  (`PrimitiveComponent.AddForce` (`self.Master`) (`KismetMathLibrary.MakeVector` 0.0 0.0 (`self.GravityDownForce`)) "None" true))

(fn `HandleInputRotation`
  (params (`Input Value` :type "Float (double-precision)") (RotationForce :type "Float (double-precision)") (VectorDir :type "Vector Structure"))
  (`PrimitiveComponent.AddTorqueInDegrees` (`self.Master`) (`KismetMathLibrary.VLerp` (0.0 0.0 0.0) (* VectorDir (* `Input Value` RotationForce)) 0.1) "None" true))

(fn `HandleRotationCompensation`
  (`PrimitiveComponent.AddTorqueInDegrees` (`self.Master`) (/ (`KismetMathLibrary.NegateVector` (`PrimitiveComponent.GetPhysicsAngularVelocityInDegrees` (`self.Master`) "None")) (`self.AngularCompensation`)) "None" true))

(fn `PosNegValue`
  (params (Value :type "Float (double-precision)") (Positive :type "Float (double-precision)") (Negative :type "Float (double-precision)"))
  (returns (`Return Value` :type "Float (double-precision)"))
  (locals (calculateResult :type "Float (double-precision)"))
  (if (> Value 0.0)
    (set `local.calculateResult` (* Value Positive))
    (return (`local.calculateResult`))
    (elif (< Value 0.0)
      (set `local.calculateResult` (* Value Negative))
      (return (`local.calculateResult`)))))

(fn `Scale6`
  (params (value :type "Vector Structure") (posX :type "Float (double-precision)") (negX :type "Float (double-precision)") (posY :type "Float (double-precision)") (negY :type "Float (double-precision)") (posZ :type "Float (double-precision)") (negZ :type "Float (double-precision)"))
  (returns (returnValue :type "Vector Structure"))
  (locals (result :type "Vector Structure"))
  (bind (_result_x _result_y _result_z) (`KismetMathLibrary.BreakVector` (`local.result`)))
  (bind _result_x_2 (`KismetMathLibrary.BreakVector` (`local.result`)))
  (bind (_result_x_3 _result_y_2 _result_z_2) (`KismetMathLibrary.BreakVector` (`local.result`)))
  (bind (_result_x_4 _result_y_3 _result_z_3) (`KismetMathLibrary.BreakVector` (`local.result`)))
  (bind (_result_x_5 _result_y_4) (`KismetMathLibrary.BreakVector` (`local.result`)))
  (bind (_result_x_6 _result_y_5) (`KismetMathLibrary.BreakVector` (`local.result`)))
  (set `local.result` value)
  (bind _return_value (`self.PosNegValue` _result_x_2 posX negX))
  (set `local.result` (`KismetMathLibrary.MakeVector` _return_value _result_y_2 _result_z_2))
  (bind _return_value_2 (`self.PosNegValue` _result_y_5 posY negY))
  (set `local.result` (`KismetMathLibrary.MakeVector` _result_x_4 _return_value_2 _result_z_3))
  (bind _return_value_3 (`self.PosNegValue` _result_z posZ negZ))
  (bind _output_get (set `local.result` (`KismetMathLibrary.MakeVector` _result_x_5 _result_y_4 _return_value_3)))
  (return _output_get))

(fn `UpdateDrag`
  (params (deltaTime :type "Float (double-precision)"))
  (locals (lv :type "Vector Structure" :default (0.0 0.0 0.0)) (lv2 :type "Float (double-precision)" :default 0.0) (Coefficient :type "Vector Structure" :default (0.0 0.0 0.0)) (NewLocalVar :type "Vector Structure"))
  (bind _localvelocity (`self.LocalVelocity`))
  (bind (_coefficient_x _coefficient_y _coefficient_z) (`KismetMathLibrary.BreakVector` (`local.Coefficient`)))
  (bind (_returnvalue_x _returnvalue_y _returnvalue_z) (`KismetMathLibrary.BreakVector` (`KismetMathLibrary.Normal` (`local.lv`))))
  (bind _returnvalue (`SceneComponent.K2_GetComponentLocation` (`self.Master`)))
  (set `local.lv` _localvelocity)
  (set `local.lv2` (`KismetMathLibrary.VSizeSquared` _localvelocity))
  ;[1 0 0 0.5] Remplacer par des variable qui seront des curves
  (bind _returnvalue_2 (`self.Scale6` (`KismetMathLibrary.Normal` (`local.lv`)) 1.0 2.0 2.0 2.0 2.0 2.0))
  (bind _output_get (set `local.Coefficient` _returnvalue_2))
  (`KismetSystemLibrary.DrawDebugLine` _returnvalue (+ _returnvalue (* (`KismetMathLibrary.VSize` _output_get) (`local.lv2`) (`KismetMathLibrary.NegateVector` (`KismetMathLibrary.Normal` (`local.lv`))))) (struct :`G` 0.384889 :`B` 1.0 :`A` 1.0))
  (`KismetSystemLibrary.DrawDebugLine` _returnvalue (+ _returnvalue (`local.lv`)) (struct :`R` 1.0 :`G` 0.101863 :`B` 0.968866 :`A` 1.0))
  (`KismetSystemLibrary.DrawDebugLine` _returnvalue (+ _returnvalue (`self.Velocity`)) (struct :`R` 1.0 :`A` 1.0))
  (`KismetSystemLibrary.PrintText` (`|FormatText` "coef:{x} y:{y} z:{z}" _coefficient_x _coefficient_y _coefficient_z) true true (struct :`R` 1.0 :`G` 0.358931 :`B` 0.005019 :`A` 1.0) -1.0 "coef")
  (`KismetSystemLibrary.PrintText` (`|FormatText` "lvl 2 x:{x}" (`local.lv2`)) true true (struct :`R` 1.0 :`G` 0.358931 :`B` 0.005019 :`A` 1.0) -1.0 "lvl2")
  (`KismetSystemLibrary.PrintText` (`|FormatText` "lvl normalize x:{x} y:{y} z:{z}" _returnvalue_x _returnvalue_y _returnvalue_z) true true (struct :`R` 1.0 :`G` 0.358931 :`B` 0.005019 :`A` 1.0) 2.0 "lvln"))

(fn `UpdateLift`
  (locals (localLiftForce :type "Vector Structure" :default (0.0 0.0 0.0)) (localYawForce :type "Vector Structure" :default (0.0 0.0 0.0)))
  (bind _master (`self.Master`))
  (bind _master_2 (`self.Master`))
  (bind _returnvalue (`SceneComponent.K2_GetComponentLocation` (`self.Master`)))
  (if (not (< (`KismetMathLibrary.VSizeSquared` (`self.LocalVelocity`)) 1.0))
    (bind _return_value (`self.CalculateLift` (`self.AngleOfAttack`) (`SceneComponent.GetRightVector` _master) (`self.LiftPower`) (`self.aoaCurve`) (`self.inducedDragCurve`)))
    (set `local.localLiftForce` _return_value)
    (bind _return_value_2 (`self.CalculateLift` (`self.AngleOfAttackYaw`) (`SceneComponent.GetUpVector` _master) (`self.RudderPower`) (`self.RudderAoACurve`) (`self.RudderInducedDragCurve`)))
    (set `local.localYawForce` _return_value_2)
    (`PrimitiveComponent.AddForce` _master_2 (`local.localLiftForce`) "None" false)
    (`PrimitiveComponent.AddForce` _master_2 (`local.localYawForce`) "None" false)
    (`KismetSystemLibrary.DrawDebugLine` _returnvalue (+ _returnvalue (`local.localLiftForce`)) (struct :`R` 0.111873 :`G` 1.0 :`A` 1.0))
    (`KismetSystemLibrary.DrawDebugLine` _returnvalue (+ _returnvalue (`local.localYawForce`)) (struct :`R` 1.0 :`G` 0.566505 :`A` 1.0))))

(fn `UserConstructionScript`)